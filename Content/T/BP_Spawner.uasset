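; BP_Spawner spawns randomly scaled BP_Bubble actors within a box around itself, setting each one's projectile speed and gravity.
; Once Start is called, a Delay loop spawns bubbles while a looping timer periodically lowers spawn delay, speed and gravity scale.
; Every second step triggers a temporary zero-delay bubble burst, during which and briefly afterward BP_Click is protected from life loss and its heart is changed.
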(event `self.ReceiveBeginPlay`
  (bind _asbp_click (cast `/Game/T/BP_Click` (`GameplayStatics.GetPlayerPawn` 0)))
  (set `self.As BP Click` _asbp_click))

(event `Start`
  (bind _returnvalue (`KismetMathLibrary.RandomFloatInRange` 0.5 2.0))
  (`KismetSystemLibrary.K2_SetTimerDelegate` (delegate `Time`) 0.5 true)
  (bind _returnvalue_2 (`|SpawnActorFromClass` "/Game/T/BP_Bubble.BP_Bubble_C" (`KismetMathLibrary.Conv_VectorToTransform` (`KismetMathLibrary.RandomPointInBoundingBox` (`self.K2_GetActorLocation`) (10.0 200.0 0.0))) "Undefined" "MultiplyWithRoot" null null :!label _label))
  (`SceneComponent.SetRelativeScale3D` (`/Game/T/BP_Bubble.Plane` _returnvalue_2) (`KismetMathLibrary.MakeVector` _returnvalue _returnvalue _returnvalue))
  (bind _projectilemovement (`/Game/T/BP_Bubble.ProjectileMovement` _returnvalue_2))
  (set `ProjectileMovementComponent.InitialSpeed` (`self.Speed`) _projectilemovement)
  (set `ProjectileMovementComponent.MaxSpeed` (`self.MaxSpeed`) _projectilemovement)
  (set `ProjectileMovementComponent.ProjectileGravityScale` (`self.Gravity`) _projectilemovement)
  (`KismetSystemLibrary.Delay` (`self.SpawnRate`))
  (goto _label))

(event `Time`
  (bind _result (`/Engine/EditorBlueprintResources/StandardMacros.IncrementInt` (`self.Seconds`))
    (:`  `
      (bind _output_get (set `self.Seconds` _result))
      (if (== _output_get 15)
        (set `self.SpawnRate` (- (`self.SpawnRate`) 0.15))
        (set `self.Speed` (- (`self.Speed`) 1.0))
        (set `self.Gravity` (- (`self.Gravity`) 0.05))
        (set `self.Seconds` 0)
        (bind _result_2 (`/Engine/EditorBlueprintResources/StandardMacros.IncrementInt` (`self.Counter`))
          (:`  `
            (set `self.Counter` _result_2)))
        (elif (== (`self.Counter`) 2)
          (`/Game/T/BP_Click.Heart Change` (`self.As BP Click`))
          (set `self.PreviousSR` (`self.SpawnRate`))
          (set `self.PreviousS` (`self.Speed`))
          (set `self.PreviousMS` (`self.MaxSpeed`))
          (set `self.PreviousG` (`self.Gravity`))
          (set `self.SpawnRate` 0.0)
          (set `self.Speed` 15.0)
          (set `self.MaxSpeed` 1000.0)
          (set `self.Gravity` -10.0)
          (set `self.Counter` 0)
          (set `/Game/T/BP_Click.DontLoseLife` true (`self.As BP Click`))
          (`KismetSystemLibrary.Delay` 5.0)
          (set `self.SpawnRate` (`self.PreviousSR`))
          (set `self.Speed` (`self.PreviousS`))
          (set `self.MaxSpeed` (`self.PreviousMS`))
          (set `self.Gravity` (`self.PreviousG`))
          (`KismetSystemLibrary.Delay` 3.0)
          (set `/Game/T/BP_Click.DontLoseLife` false (`self.As BP Click`))
          (`/Game/T/BP_Click.HeartBack` (`self.As BP Click`)))))))

(fn `UserConstructionScript`)