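; BP_Bubble is a bubble actor that pops when its Plane mesh is touched.
; It caches the BP_Click player pawn on BeginPlay and calls its CallPopped on the first touch, guarded by a DoOnce.
; The pop swaps to a burst material, plays a randomly selected pop sound, then destroys the actor after a short delay.
; A mouse click on the plane only prints a debug string.
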(event `self.Plane.OnClicked`
  (params (TouchedComponent :type "PrimitiveComponent Object Reference") (ButtonPressed :type "Key Structure"))
  (`KismetSystemLibrary.PrintString` "Hello"))

(event `self.ReceiveBeginPlay`
  (bind _asbp_click (cast `/Game/T/BP_Click` (`GameplayStatics.GetPlayerPawn` 0)))
  (set `self.As BP Click` _asbp_click))

(event `self.ReceiveActorOnClicked`
  (params (ButtonPressed :type "Key Structure")))

(event `self.Plane.OnInputTouchBegin`
  (params (FingerIndex :type "ETouchIndex Enum" :default "Touch1") (TouchedComponent :type "PrimitiveComponent Object Reference"))
  (bind _audio (`self.Audio`))
  (`/Engine/EditorBlueprintResources/StandardMacros.DoOnce` false
    (:`Completed`
      (`/Game/T/BP_Click.Popped` (`self.As BP Click`))
      (`PrimitiveComponent.SetMaterial` (`self.Plane`) 0 "/Game/T/Assets/M_BubblePop.M_BubblePop")
      (`AudioComponent.SetSound` _audio (select `int` (`KismetMathLibrary.RandomIntegerInRange` 0 5) :`0` "/Game/T/Sounds/Pop_4.Pop_4" :`1` "/Game/T/Sounds/Pop_2.Pop_2" :`2` "/Game/T/Sounds/Pop_3.Pop_3" :`3` "/Game/T/Sounds/Pop_4.Pop_4" :`4` "/Game/T/Sounds/Pop_5.Pop_5" :`5` "/Game/T/Sounds/Pop_6.Pop_6" :!type "SoundBase Object Reference"))
      (`AudioComponent.Play` _audio 0.0)
      (`KismetSystemLibrary.Delay` 0.4)
      (`self.K2_DestroyActor`))))

(fn `UserConstructionScript`)