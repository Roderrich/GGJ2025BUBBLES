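; BP_Click is an actor that manages score and lives for what appears to be a click-to-pop game.
; On BeginPlay it shows the mouse cursor, adds the screen widget and binds Pointup to Popped, adding and printing points.
; LoseLife decrements lives unless DontLoseLife is set, then at zero clears widgets, pauses and shows the score widget.
; HeartBack and HeartChange switch an Image index between two values.
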(event `self.ReceiveBeginPlay`
  (set `PlayerController.bShowMouseCursor` true (`PlayerState.GetPlayerController` (`GameplayStatics.GetPlayerState` 0)))
  (bind _returnvalue (`|CreateWidget` "/Game/T/UI/WBP_Screen.WBP_Screen_C"))
  (`UserWidget.AddToViewport` _returnvalue 0)
  (add `self.Popped` (delegate `Pointup`)))

(event `Pointup`
  (bind _output_get (set `self.Points` (+ (`self.Points`) 10.0)))
  (`KismetSystemLibrary.PrintString` (`KismetStringLibrary.Conv_DoubleToString` _output_get)))

(event `LoseLife`
  (if (not (`self.DontLoseLife`))
    (bind _result (`/Engine/EditorBlueprintResources/StandardMacros.DecrementInt` (`self.Life`))
      (:`  `
        (bind _output_get (set `self.Life` _result))
        (if (== _output_get 0)
          (`WidgetLayoutLibrary.RemoveAllWidgets`)
          (`GameplayStatics.SetGamePaused` true)
          (bind _returnvalue (`|CreateWidget` "/Game/T/UI/WBP_Score.WBP_Score_C"))
          (`UserWidget.AddToViewport` _returnvalue 0))))))

(event `HeartBack`
  (set `self.Image` (`self.1`)))

(event `Heart Change`
  (set `self.Image` (`self.2`)))

(fn `UserConstructionScript`)